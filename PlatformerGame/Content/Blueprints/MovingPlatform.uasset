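; MovingPlatform is an actor that shuttles its static mesh back and forth between two positions indefinitely.
; BeginPlay stores the actor location as StartPosition and first targets EndPosition.
; A latent MoveComponentTo moves the mesh over MoveSpeed as a duration, then flips the target and loops.
; Both positions feed the relative-location target, although StartPosition is captured in world space.
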(event `self.ReceiveBeginPlay`
  (set `self.StartPosition` (`self.K2_GetActorLocation`))
  (set `self.TargetPosition` (`self.EndPosition`))
  (`KismetSystemLibrary.MoveComponentTo` (`self.StaticMesh`) (`self.TargetPosition`) (struct) false false (`self.MoveSpeed`) :!label _label)
  (if (== (`self.TargetPosition`) (`self.StartPosition`))
    (set `self.TargetPosition` (`self.EndPosition`))
    (goto _label)
    (else
      (set `self.TargetPosition` (`self.StartPosition`))
      (goto _label))))

(fn `UserConstructionScript`)