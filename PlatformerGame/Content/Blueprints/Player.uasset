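; Player pawn Blueprint that handles movement, jumping, score and end-of-game screens.
; Axis inputs feed AddMovementInput along actor forward and right, while jump applies upward force to the StaticMesh only when Grounded.
; Grounded clears on jump and resets when a hit normal points almost exactly up.
; BeginPlay creates the game UI that AddScore updates; GameOver and GameWin show the end screen and mouse cursor.
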(event `InputAction|Jump`
  (params (Key :type "Key Structure"))
  ;[1 1 1] Jumping
  (:`Pressed`
    (if (`self.Grounded`)
      (`PrimitiveComponent.AddForce` (`self.StaticMesh`) (* (`KismetMathLibrary.Vector_Up`) (`self.JumpForce`)) "None" false)
      (set `self.Grounded` false))))

(event `InputAxis|Move_ForwardBackward`
  (params (AxisValue :type "Float (single-precision)"))
  ;[1 1 1] Moving
  (`self.AddMovementInput` (`self.GetActorForwardVector`) AxisValue))

(event `InputAxis|Move_LeftRight`
  (params (AxisValue :type "Float (single-precision)"))
  ;[1 1 1] Moving
  (`self.AddMovementInput` (`self.GetActorRightVector`) AxisValue))

(event `self.ReceiveHit`
  (params (MyComp :type "PrimitiveComponent Object Reference") (Other :type "Actor Object Reference") (OtherComp :type "PrimitiveComponent Object Reference") (bSelfMoved :type Boolean) (HitLocation :type "Vector Structure") (HitNormal :type "Vector Structure") (NormalImpulse :type "Vector Structure") (Hit :type "HitResult Structure (by ref)"))
  ;[1 1 1] Ground Checking
  (if (== HitNormal (0.0 0.0 1.0))
    (set `self.Grounded` true)))

(event `self.ReceiveBeginPlay`
  (bind _returnvalue (`|CreateWidget` "/Game/Blueprints/GameUI.GameUI_C"))
  (`UserWidget.AddToViewport` _returnvalue 0)
  (set `self.GameUI` _returnvalue))

(fn `AddScore`
  (params (`Score to Add` :type Integer))
  (bind _output_get (set `self.Score` (+ `Score to Add` (`self.Score`))))
  (`/Game/Blueprints/GameUI.SetScore` (`self.GameUI`) _output_get))

(fn `GameOver`
  (bind _returnvalue (`|CreateWidget` "/Game/Blueprints/EndGameUI.EndGameUI_C"))
  (`UserWidget.AddToViewport` _returnvalue 0)
  (`/Game/Blueprints/EndGameUI.SetEndScreen` _returnvalue false)
  (set `PlayerController.bShowMouseCursor` true (`GameplayStatics.GetPlayerController` 0)))

(fn `GameWin`
  (bind _returnvalue (`|CreateWidget` "/Game/Blueprints/EndGameUI.EndGameUI_C"))
  (`UserWidget.AddToViewport` _returnvalue 0)
  (`/Game/Blueprints/EndGameUI.SetEndScreen` _returnvalue true)
  (set `PlayerController.bShowMouseCursor` true (`GameplayStatics.GetPlayerController` 0)))

(fn `UserConstructionScript`)